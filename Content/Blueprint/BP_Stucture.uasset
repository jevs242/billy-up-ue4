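; BP_Stucture is an actor with a floor that slides back and forth along its relative Y axis, like a moving platform.
; Tick offsets the Floor component by Speed scaled by delta time, keeping motion frame-rate independent.
; When the Box component begins overlapping WallRight or WallLeft, Speed flips sign to reverse direction.
; Hits on the Floor only print a debug "Hello" message.
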(event OnComponentHit(Floor)
  (params (HitComponent :type Primitive%20Component%20Object%20Reference) (OtherActor :type Actor%20Object%20Reference) (OtherComp :type Primitive%20Component%20Object%20Reference) (NormalImpulse :type Vector :default "0, 0, 0") (Hit :type Hit%20Result%20Structure%20%28by%20ref%29))
  (Development|PrintString "Hello"))

(event OnComponentBeginOverlap(Box)
  (params (OverlappedComponent :type Primitive%20Component%20Object%20Reference) (OtherActor :type Actor%20Object%20Reference) (OtherComp :type Primitive%20Component%20Object%20Reference) (OtherBodyIndex :type Integer) (bFromSweep :type Boolean) (SweepResult :type Hit%20Result%20Structure%20%28by%20ref%29))
  (if (== OtherComp (Variables|Default|GetWallRight))
    (Variables|Default|SetSpeed (* (Variables|Default|GetSpeed) -1.0))
    (elif (== OtherComp (Variables|Default|GetWallLeft))
      (Variables|Default|SetSpeed (* (Variables|Default|GetSpeed) -1.0)))))

(event EventBeginPlay)

(event Collision|EventActorBeginOverlap
  (params (OtherActor :type Actor%20Object%20Reference)))

(event EventTick
  (params (DeltaSeconds :type Float%20%28single-precision%29))
  (bind _floor (Variables|Default|GetFloor))
  (bind _relativelocation (Variables|/Script/Engine.SceneComponent|GetRelativeLocation _floor))
  (Transformation|SetRelativeLocation _floor (Math|Vector|MakeVector (.x _relativelocation) (+ (* DeltaSeconds (Variables|Default|GetSpeed)) (.y _relativelocation)) (.z _relativelocation)) false false))

(fn ConstructionScript)