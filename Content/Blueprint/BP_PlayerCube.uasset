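; BP_PlayerCube is the player cube, which owns its UI, background music and blinking eyes.
; BeginPlay creates the HUD and main menu, hides the HUD, starts the music and launches a self-calling EyeLash loop that periodically squashes the eyes' Z scale.
; Tick pins the camera boom's world Y at zero while keeping X and Z.
; Escape hides a visible HUD and opens a new pause widget.
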(event Custom|Visibility%20HUD
  (params (InVisibility :type ESlateVisibility%20Enum :default "Visible"))
  (Widget|SetVisibility (Variables|Default|GetHUD) InVisibility))

(event Custom|EyeLash
  (bind _eyer (Variables|Default|GetEyeR))
  (bind _eyel (Variables|Default|GetEyeL))
  (bind _eyer_2 (Variables|Default|GetEyeR))
  (bind _relativescale3d (Variables|/Script/Engine.SceneComponent|GetRelativeScale3D _eyer))
  (bind _relativescale3d_2 (Variables|/Script/Engine.SceneComponent|GetRelativeScale3D _eyel))
  (bind _relativescale3d_3 (Variables|/Script/Engine.SceneComponent|GetRelativeScale3D _eyer_2))
  (bind _relativescale3d_4 (Variables|/Script/Engine.SceneComponent|GetRelativeScale3D _eyer))
  (Utilities|FlowControl|Delay 1.0)
  (Transformation|SetRelativeScale3D _eyer (Math|Vector|MakeVector (.x _relativescale3d_4) (.y _relativescale3d_4) 0.056166))
  (Transformation|SetRelativeScale3D (Variables|Default|GetEyeL) (Math|Vector|MakeVector (.x _relativescale3d) (.y _relativescale3d) 0.056166))
  (Utilities|FlowControl|Delay 0.2)
  (Transformation|SetRelativeScale3D _eyer_2 (Math|Vector|MakeVector (.x _relativescale3d_3) (.y _relativescale3d_3) (Variables|Default|GetScaleZ)))
  (Transformation|SetRelativeScale3D (Variables|Default|GetEyeL) (Math|Vector|MakeVector (.x _relativescale3d_2) (.y _relativescale3d_2) (Variables|Default|GetScaleZ)))
  (CallFunction|EyeLash))

(event EventBeginPlay
  (bind _returnvalue (UserInterface|CreateWidget "/Game/Blueprint/Wideget/WBP_HUD.WBP_HUD_C"))
  (bind _output_get (Variables|Default|SetHUD _returnvalue))
  (UserInterface|Viewport|AddtoPlayerScreen _output_get)
  (bind _returnvalue_2 (UserInterface|CreateWidget "/Game/Blueprint/Wideget/WBP_Menu.WBP_Menu_C"))
  (bind _output_get_2 (Variables|Default|SetMenu _returnvalue_2))
  (UserInterface|Viewport|AddtoPlayerScreen _output_get_2)
  (CallFunction|VisibilityHUD "Hidden")
  (bind _returnvalue_3 (Audio|CreateSound2D "/Game/Sound/Moody_Cyberpunk_Synth_-_Midnight____Royalty_Free_No_Copyright_Background_Music_Cue.Moody_Cyberpunk_Synth_-_Midnight____Royalty_Free_No_Copyright_Background_Music_Cue" 1.0 1.0 0.0 0))
  (bind _output_get_3 (Variables|Default|SetMusic _returnvalue_3))
  (Audio|Components|Audio|Play _output_get_3 0.0)
  (Variables|Default|SetScaleZ (.z (Variables|/Script/Engine.SceneComponent|GetRelativeScale3D (Variables|Default|GetEyeL))))
  (CallFunction|EyeLash))

(event Collision|EventActorBeginOverlap
  (params (OtherActor :type Actor%20Object%20Reference)))

(event EventTick
  (params (DeltaSeconds :type Float%20%28single-precision%29))
  (bind _cameraboom (Variables|Default|GetCameraBoom))
  (bind _returnvalue (Transformation|GetWorldLocation _cameraboom))
  (Transformation|SetWorldLocation _cameraboom (Math|Vector|MakeVector (.x _returnvalue) 0.0 (.z _returnvalue)) false false))

(event Input|KeyboardEvents|Escape
  (params (Key :type Key%20Structure :default "None"))
  (:Pressed
    (if (Utilities|Enum|Equal(Enum) (Widget|GetVisibility (Variables|Default|GetHUD)) "Visible")
      (CallFunction|VisibilityHUD "Hidden")
      (bind _returnvalue (UserInterface|CreateWidget "/Game/Blueprint/Wideget/WBP_Pause.WBP_Pause_C"))
      (UserInterface|Viewport|AddtoPlayerScreen _returnvalue))))

(fn ConstructionScript)